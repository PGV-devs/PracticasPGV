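; BP_Missle is a missile projectile actor in the AreaAttack folder that launches along its local downward axis and removes itself on impact or at maximum range.
; BeginPlay stores the start location and sets the MissleMovement velocity, while Tick destroys the actor once it travels beyond MissleRange.
; CollisionBox overlaps destroy it on any EnemySPLine_Parent child or the Landscape, with no damage applied in this Blueprint.
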(event `self.ReceiveBeginPlay`
  (set `self.StartLocation` (`self.K2_GetActorLocation`))
  (`ProjectileMovementComponent.SetVelocityInLocalSpace` (`self.MissleMovement`) (0.0 0.0 -500.0)))

(event `self.ReceiveTick`
  (params (DeltaSeconds :type "Float (single-precision)"))
  (if (> (`KismetMathLibrary.VSize` (- (`self.StartLocation`) (`self.K2_GetActorLocation`))) (`self.MissleRange`))
    (`/Engine/EditorBlueprintResources/StandardMacros.DoOnce` false
      (:`Completed`
        (`self.K2_DestroyActor`)))))

(event `self.CollisionBox.OnComponentBeginOverlap`
  (params (OverlappedComponent :type "PrimitiveComponent Object Reference") (OtherActor :type "Actor Object Reference") (OtherComp :type "PrimitiveComponent Object Reference") (OtherBodyIndex :type Integer) (bFromSweep :type Boolean) (SweepResult :type "HitResult Structure (by ref)"))
  (cast `/Game/Blueprints/Enemies/EnemySPLine_Parent` OtherActor ; Elige como objetivo cualquier tipo de bicho\nya que castea al blueprint padre de los bichos
    (:`then`
      (`/Engine/EditorBlueprintResources/StandardMacros.DoOnce` false
        (:`Completed`
          (`self.K2_DestroyActor`))))
    (:`CastFailed`
      (cast `Landscape` OtherActor)
      (`self.K2_DestroyActor`))))

(fn `UserConstructionScript`)