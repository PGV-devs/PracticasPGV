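; BP_EnemySpawner spawns the bugs of a level's first wave, one at a time on a looping timer.
; Each tick it reads the next type index from the level controller's WaveP1 array and spawns that BugTypes class at its own location.
; It casts the pawn to CharacterSPLine_Parent to assign the controller's first spline path and a fixed speed.
; Once the spawn count reaches the wave's length, it clears the timer.
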(event `self.ReceiveBeginPlay`
  (bind _returnvalue (`KismetSystemLibrary.K2_SetTimerDelegate` (delegate `SpawnEnemy`) 5.0 true)) ; Dispara el evento cada Time segundos. \nSi no se pone Loopìng a true, sólo se \nejecuta una vez.
  (set `self.EnemySpawnTimerHandler` _returnvalue) ; Permite modificar el timer mediante otras funciones
)

(event `SpawnEnemy`
  (set `self.AmountOfEnemysToSpawn` (`KismetArrayLibrary.Array_Length` (`/Game/Blueprints/BP_LevelController.WaveP1` (`self.LevelControllerRef`)))) ; inicializamos la cantiadad de enemigos a spawnear con el tamaño del array
  (bind _returnvalue (`AIBlueprintHelperLibrary.SpawnAIFromClass` (`|GetArrayItem` (`self.BugTypes`) (`|GetArrayItem` (`/Game/Blueprints/BP_LevelController.WaveP1` (`self.LevelControllerRef`)) (`self.AmountOfEnemysSpawned`))) null (`self.K2_GetActorLocation`) (struct) false null)) ; Spawnea un bicho del tipo generado
  (bind _ascharacter_spline_parent (cast `/Game/Blueprints/Characters/CharacterSPLine_Parent` _returnvalue)) ; Casteo a Spline Parent para poder asignarle el \nSpline Parent y la velocidad. Si no se realiza \nel casting no se puede acceder a los atributos.
  (set `/Game/Blueprints/Characters/CharacterSPLine_Parent.SPLineRef` (`|GetArrayItem` (`/Game/Blueprints/BP_LevelController.Paths` (`self.LevelControllerRef`))) _ascharacter_spline_parent)
  (set `/Game/Blueprints/Characters/CharacterSPLine_Parent.CharacterSpeed` 300.0 _ascharacter_spline_parent)
  (bind _result (`/Engine/EditorBlueprintResources/StandardMacros.IncrementInt` (`self.AmountOfEnemysSpawned`)) ; Contador de enemigos spawneados
    (:`  `
      (if (>= _result (`self.AmountOfEnemysToSpawn`))
        (`KismetSystemLibrary.K2_ClearAndInvalidateTimerHandle` (`self.EnemySpawnTimerHandler`)) ; Se paran de Spawnear enemigos
      ))))

(fn `UserConstructionScript`)