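; Level controller that runs tower construct mode and the end-of-game screens for a tower defense level.
; Construct mode shows BP_Tiles and a type-colored preview, which Tick snaps to CursorTile or a ground-plane mouse projection, flagging validity.
; SpawnTower spawns the selected class at the preview, then exits construct mode, destroying preview and cursor tile.
; Victory and GameOver pause the game and show the EndGame widget.
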(event `self.ReceiveBeginPlay`)

(event `self.ReceiveTick`
  (params (DeltaSeconds :type "Float (single-precision)"))
  (bind _returnvalue (`KismetSystemLibrary.IsValid` (`self.CursorTile`)))
  (if (`self.ConstructMode`)
    (`self.ToggleValidPreview` _returnvalue)
    (if _returnvalue
      (`self.K2_SetActorLocation` (`self.TowerPreview`) (`SceneComponent.K2_GetComponentLocation` (`/Game/Blueprints/Tiles/BP_Tile.StaticMesh` (`self.CursorTile`))) false false)
      (else
        (bind _mouse_location (`self.GetMouseLocation`))
        (`self.K2_SetActorLocation` (`self.TowerPreview`) _mouse_location false false)))))

(fn `Create End Game `
  (returns (EndGameWidget :type "/Game/HUD/EndGame Object Reference"))
  (locals (`End Game Widget` :type "/Game/HUD/EndGame Object Reference"))
  (bind _returnvalue (`|CreateWidget` "/Game/HUD/EndGame.EndGame_C"))
  (bind _output_get (set `local.End Game Widget` _returnvalue))
  (`Widget.SetVisibility` _output_get "Visible")
  (`UserWidget.AddToViewport` (`local.End Game Widget`) 2)
  (return (`local.End Game Widget`)))

(fn `Enter Construct Mode`
  (params (`Tower Type` :type Integer))
  (locals (Type :type Integer))
  (set `self.TowerType` `Tower Type`)
  (set `self.ConstructMode` true)
  (bind _returnvalue (`|SpawnActorFromClass` "/Game/Blueprints/Towers/BP_TowerPreview.BP_TowerPreview_C" (`KismetMathLibrary.MakeTransform` (0.0 0.0 0.0) (struct) (`self.ScaleTowers`)) "Undefined" "OverrideRootScale" null null))
  (set `self.TowerPreview` _returnvalue)
  (`self.Set Material From Type`)
  (`self.Toggle Tiles` (`self.ConstructMode`)))

(fn `Exit Construct Mode`
  (set `self.ConstructMode` false)
  (`self.K2_DestroyActor` (`self.TowerPreview`))
  (`self.K2_DestroyActor` (`self.CursorTile`))
  (`self.Toggle Tiles` (`self.ConstructMode`)))

(fn `Game Over`
  (locals (EndGameWidget :type "/Game/HUD/EndGame Object Reference"))
  (`GameplayStatics.SetGamePaused` true)
  (bind _endgamewidget (`self.Create End Game `))
  (`Widget.SetVisibility` (`/Game/HUD/EndGame.GameOver` _endgamewidget) "Visible"))

(fn `GetMouseLocation`
  (returns (`Mouse Location` :type "Vector Structure"))
  (bind (_worldlocation _worlddirection) (`PlayerController.DeprojectMousePositionToWorld` (`GameplayStatics.GetPlayerController` 0)))
  (return (+ (+ _worldlocation (* (* _worlddirection (/ (.z _worldlocation) (.z _worlddirection))) -1.0)) (0.0 0.0 35.0))))

(fn `Set Material From Type`
  (locals (Material :type "MaterialInstance Object Reference"))
  (switch `int` (`self.TowerType`)
    (:`0`
      (set `local.Material` "/Game/Materiales/Glass/GLASS_T1.GLASS_T1"))
    (:`1`
      (set `local.Material` "/Game/Materiales/Glass/GLASS_T2.GLASS_T2"))
    (:`2`
      (set `local.Material` "/Game/Materiales/Glass/GLASS_T3.GLASS_T3")))
  (set `/Game/Blueprints/Towers/BP_TowerPreview.Tower Material` (`local.Material`) (`self.TowerPreview`)))

(fn `SpawnTower`
  (locals (TowerClass :type "Actor Class Reference" :default "BlueprintGeneratedClass'/Game/Blueprints/Towers/Tower.Tower_C'"))
  (switch `int` (`self.TowerType`)
    (:`0`
      (set `local.TowerClass` "/Game/Blueprints/Towers/Tower_SimpleTurret.Tower_SimpleTurret_C"))
    (:`1`
      (set `local.TowerClass` "/Game/Blueprints/Towers/Tower_Mortar.Tower_Mortar_C"))
    (:`2`
      (set `local.TowerClass` "/Game/Blueprints/Towers/Tower_GreatTurret.Tower_GreatTurret_C")))
  (`|SpawnActorFromClass` (`local.TowerClass`) (`self.GetTransform` (`self.TowerPreview`)) "AlwaysSpawn" "OverrideRootScale" null null)
  (`self.Exit Construct Mode`))

(fn `Toggle Tiles`
  (params (ConstructMode :type Boolean))
  (locals (`Construct Mode` :type Boolean))
  (set `local.Construct Mode` ConstructMode)
  (bind _outactors (`GameplayStatics.GetAllActorsOfClass` "/Game/Blueprints/Tiles/BP_Tile.BP_Tile_C"))
  (for _array_element _outactors
    (set `/Game/Blueprints/Tiles/BP_Tile.Visible` (`self.ConstructMode`) _array_element)))

(fn `ToggleValidPreview`
  (params (Valid :type Boolean))
  (set `/Game/Blueprints/Towers/BP_TowerPreview.Valid` Valid (`self.TowerPreview`)))

(fn `UserConstructionScript`)

(fn `Victory`
  (`GameplayStatics.SetGamePaused` true)
  (bind _endgamewidget (`self.Create End Game `))
  (`Widget.SetVisibility` (`/Game/HUD/EndGame.YouWin` _endgamewidget) "Visible"))