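; BP_Base is a damageable actor with hit points and an attached enemy HP widget.
; On BeginPlay it fills its current HP to the maximum and passes itself to the WB_HPEnemy widget as its parent object.
; ReceiveDamage subtracts incoming damage from current HP and destroys the actor once HP reaches zero or below.
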(event `self.ReceiveBeginPlay`
  (set `self.CurrentHP` (`self.HP_MAX`))
  (bind _aswb_hpenemy (cast `/Game/HUD/WB_HPEnemy` (`WidgetComponent.GetUserWidgetObject` (`self.WidgetHPEnemy`))))
  (set `/Game/HUD/WB_HPEnemy.Parent Object` self _aswb_hpenemy))

(fn `ReceiveDamage`
  (params (Damage :type "Float (double-precision)"))
  (locals (NewHP :type "Float (double-precision)"))
  (bind _output_get (set `local.NewHP` (- (`self.CurrentHP`) Damage)))
  (if (<= _output_get 0.0)
    (set `self.CurrentHP` 0.0)
    (`self.K2_DestroyActor`)
    (else
      (set `self.CurrentHP` (`local.NewHP`)))))

(fn `UserConstructionScript`)