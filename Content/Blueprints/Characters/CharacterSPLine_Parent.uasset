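; Parent Blueprint for characters that travel along a referenced spline actor, with an empty event graph.
; AddMovement advances the stored distance by speed times delta seconds, resetting to zero when the next step lands within a small tolerance of the spline's length.
; UpdateLocationAndRotation places the actor at that distance in world space with a fixed height offset, matching the spline's rotation.
; Neither function is called within this Blueprint.
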(fn `AddMovement`
  (bind _returnvalue (+ (`self.DistanceAlongSPLine`) (* (`self.CharacterSpeed`) (`GameplayStatics.GetWorldDeltaSeconds`))))
  (if (`KismetMathLibrary.NearlyEqual_FloatFloat` _returnvalue (`SplineComponent.GetSplineLength` (`/Game/Blueprints/Splines/PR2/PathSPLine.Spline` (`self.SPLineRef`))) 20.0)
    (set `self.DistanceAlongSPLine` 0.0)
    (else
      (set `self.DistanceAlongSPLine` _returnvalue))))

(fn `UpdateLocationAndRotation`
  (bind (_returnvalue_x _returnvalue_y _returnvalue_z) (`KismetMathLibrary.BreakVector` (`SplineComponent.GetLocationAtDistanceAlongSpline` (`/Game/Blueprints/Splines/PR2/PathSPLine.Spline` (`self.SPLineRef`)) (`self.DistanceAlongSPLine`) "World")))
  (`self.K2_SetActorLocationAndRotation` (`KismetMathLibrary.MakeVector` _returnvalue_x _returnvalue_y (+ _returnvalue_z 110.0)) (`SplineComponent.GetRotationAtDistanceAlongSpline` (`/Game/Blueprints/Splines/PR2/PathSPLine.Spline` (`self.SPLineRef`)) (`self.DistanceAlongSPLine`) "World")))

(fn `UserConstructionScript`)