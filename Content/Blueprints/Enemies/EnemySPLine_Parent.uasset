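; Parent enemy for a tower defense game that follows a spline path, attacks towers or the base, and has a health bar widget.
; AddMovement and UpdateLocationAndRotation handle spline travel but are not called within this Blueprint.
; Capsule overlap sets the target and starts attacking; a Delay on Tick paces damage by AttackSpeed.
; Invalid targets return it to running, or idle at path end; zero HP destroys it immediately, leaving the death animation unused.
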(event `self.ReceiveBeginPlay`
  (set `self.CurrentHP` (`self.HP_MAX`)) ; Inicializar Current HP
  ;[1 1 1] Asignar Barra Vida
  (bind _aswb_hpenemy (cast `/Game/HUD/WB_HPEnemy` (`WidgetComponent.GetUserWidgetObject` (`self.WidgetHPEnemy`))))
  (set `/Game/HUD/WB_HPEnemy.Parent Object` self _aswb_hpenemy))

(event `self.ReceiveTick`
  (params (DeltaSeconds :type "Float (single-precision)"))
  (if (`|EnumEquality` (`self.State`) "NewEnumerator1")
    (`KismetSystemLibrary.Delay` (`self.AttackSpeed`))
    (`self.ApplyDamage`)))

(event `self.CapsuleComponent.OnComponentBeginOverlap`
  (params (OverlappedComponent :type "PrimitiveComponent Object Reference") (OtherActor :type "Actor Object Reference") (OtherComp :type "PrimitiveComponent Object Reference") (OtherBodyIndex :type Integer) (bFromSweep :type Boolean) (SweepResult :type "HitResult Structure (by ref)"))
  (set `self.Other Actor` OtherActor)
  (set `self.Other Comp` OtherComp)
  (bind _astower (cast `/Game/Blueprints/Towers/Tower` (`self.Other Actor`))
    (:`then`
      (cast `BoxComponent` (`self.Other Comp`))
      (set `self.Target` _astower)
      (set `self.TargetType` "NewEnumerator0"))
    (:`CastFailed`
      (bind _asbp_base (cast `/Game/Blueprints/Base/BP_Base` (`self.Other Actor`)))
      (set `self.Target` _asbp_base)
      (set `self.TargetType` "NewEnumerator1")))
  (`self.PlayAttackAnimation`))

(fn `AddMovement`
  (bind _returnvalue (+ (`self.DistanceAlongPath`) (* (`self.CharacterSpeed`) (`GameplayStatics.GetWorldDeltaSeconds`))))
  (if (`|EnumEquality` (`self.State`) "NewEnumerator0")
    (if (`KismetMathLibrary.NearlyEqual_FloatFloat` (`SplineComponent.GetSplineLength` (`/Game/Blueprints/Splines/PathSPLine.Spline` (`self.Path`))) _returnvalue 30.0)
      (set `self.endOfPath` true)
      (`self.PlayIdleAnimation`)
      (else
        (set `self.DistanceAlongPath` _returnvalue)))))

(fn `ApplyDamage`
  (`/Engine/EditorBlueprintResources/StandardMacros.IsValid` (`self.Target`)
    (:`Is Valid`
      (if (`|EnumEquality` (`self.TargetType`) "NewEnumerator0")
        ;[1 1 1] Attack Tower
        (bind _astower (cast `/Game/Blueprints/Towers/Tower` (`self.Target`)))
        (`/Game/Blueprints/Towers/Tower.receiveDamage` _astower (`self.Damage`))
        (else
          ;[1 1 1] Attack Base
          (bind _asbp_base (cast `/Game/Blueprints/Base/BP_Base` (`self.Target`)))
          (`/Game/Blueprints/Base/BP_Base.ReceiveDamage` _asbp_base (`self.Damage`)))))
    (:`Is Not Valid`
      (if (`self.endOfPath`)
        (`self.PlayIdleAnimation`)
        (else
          (set `self.State` "NewEnumerator0")
          (`SkeletalMeshComponent.PlayAnimation` (`self.Mesh`) "/Game/Models/Spider/animations/Run_ani_vor.Run_ani_vor" true))))))

(fn `Die`
  (set `self.State` "NewEnumerator2")
  (`self.K2_DestroyActor`))

(fn `PlayAttackAnimation`
  (set `self.State` "NewEnumerator1")
  (`SkeletalMeshComponent.PlayAnimation` (`self.Mesh`) "/Game/Models/Spider/animations/Attack.Attack" true)
  (`SkeletalMeshComponent.SetPlayRate` (`self.Mesh`) (/ 1.0 (`self.AttackSpeed`))))

(fn `PlayIdleAnimation`
  (set `self.State` "NewEnumerator3")
  (`SkeletalMeshComponent.PlayAnimation` (`self.Mesh`) "/Game/Models/Spider/animations/Warte_pose.Warte_pose" true))

(fn `ReceiveDamage`
  (params (Damage :type "Float (double-precision)"))
  (returns (isDead :type Boolean))
  (locals (newHP :type "Float (double-precision)" :default 0.0))
  (bind _output_get (set `local.newHP` (- (`self.CurrentHP`) Damage)))
  (if (<= _output_get 0.0)
    (set `self.CurrentHP` 0.0)
    (`self.Die`)
    (return true)
    (else
      (set `self.CurrentHP` (`local.newHP`))
      (return false))))

(fn `UpdateLocationAndRotation`
  (bind (_returnvalue_x _returnvalue_y _returnvalue_z) (`KismetMathLibrary.BreakVector` (`SplineComponent.GetLocationAtDistanceAlongSpline` (`/Game/Blueprints/Splines/PathSPLine.Spline` (`self.Path`)) (`self.DistanceAlongPath`) "World")))
  (`self.K2_SetActorLocationAndRotation` (`KismetMathLibrary.MakeVector` _returnvalue_x _returnvalue_y (+ _returnvalue_z 110.0)) (`SplineComponent.GetRotationAtDistanceAlongSpline` (`/Game/Blueprints/Splines/PathSPLine.Spline` (`self.Path`)) (`self.DistanceAlongPath`) "World")))

(fn `UserConstructionScript`)