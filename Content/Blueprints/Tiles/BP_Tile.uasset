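; BP_Tile is a clickable tile marking a spot where a tower can be placed.
; Every Tick it sets its glass material to transparent when hidden, blue when available, or red when taken.
; On hover it registers itself as CursorTile on the BP_LevelController found at BeginPlay, clearing it on cursor exit.
; Clicking a visible, available tile marks it unavailable and calls SpawnTower on that controller.
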(event `self.ReceiveBeginPlay`
  (bind _returnvalue (`GameplayStatics.GetPlayerController` 0))
  (set `PlayerController.bEnableMouseOverEvents` true _returnvalue) ; Para detectar Mouse Over
  (set `PlayerController.bEnableClickEvents` true _returnvalue)
  (bind _outactors (`GameplayStatics.GetAllActorsOfClass` "/Game/Blueprints/BP_LevelController.BP_LevelController_C")) ; Para obtener el Level Controller
  (for _array_element _outactors
    (set `self.Level Controller Ref` _array_element)))

(event `self.ReceiveTick`
  (params (DeltaSeconds :type "Float (single-precision)"))
  (if (`self.Visible`)
    (if (`self.Available`)
      (`PrimitiveComponent.SetMaterial` (`self.StaticMesh`) 0 "/Game/Materiales/Glass/M_Glass_Blue.M_Glass_Blue")
      (else
        (`PrimitiveComponent.SetMaterial` (`self.StaticMesh`) 0 "/Game/Materiales/Glass/M_Glass_Red.M_Glass_Red")))
    (else
      (`PrimitiveComponent.SetMaterial` (`self.StaticMesh`) 0 "/Game/Materiales/Glass/M_Glass_Transparent.M_Glass_Transparent"))))

(event `self.ReceiveActorBeginCursorOver`
  (if (`self.Visible`)
    (if (`self.Available`)
      (set `/Game/Blueprints/BP_LevelController.CursorTile` self (`self.Level Controller Ref`)))))

(event `self.ReceiveActorEndCursorOver`
  (if (`self.Visible`)
    (set `/Game/Blueprints/BP_LevelController.CursorTile` null (`self.Level Controller Ref`))))

(event `self.ReceiveActorOnClicked`
  (params (ButtonPressed :type "Key Structure"))
  (if (`self.Visible`)
    (if (`self.Available`)
      (set `self.Available` false)
      (`/Game/Blueprints/BP_LevelController.SpawnTower` (`self.Level Controller Ref`)))))

(fn `UserConstructionScript`)