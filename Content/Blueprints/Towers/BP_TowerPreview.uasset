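; BP_TowerPreview is a three-part tower preview actor that shows whether it is currently valid, presumably for placement.
; Every Tick it reads the Valid flag and picks either TowerMaterial or the GLASS_INVALID material.
; ChangeMaterial stores the chosen material and applies it to the base, body and head meshes.
; The flag is not set within this Blueprint, and the material is reapplied each frame even when unchanged.
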(event `self.ReceiveBeginPlay`)

(event `self.ReceiveTick`
  (params (DeltaSeconds :type "Float (single-precision)"))
  (if (`self.Valid`)
    (`self.Change Material` (`self.Tower Material`))
    (else
      (`self.Change Material` "/Game/Materiales/Glass/GLASS_INVALID.GLASS_INVALID"))))

(fn `Change Material`
  (params (Material :type "MaterialInstance Object Reference"))
  (locals (`Material ` :type "MaterialInstance Object Reference"))
  (set `local.Material ` Material)
  (`PrimitiveComponent.SetMaterial` (`self.TowerBase`) 0 (`local.Material `))
  (`PrimitiveComponent.SetMaterial` (`self.TowerBody`) 0 (`local.Material `))
  (`PrimitiveComponent.SetMaterial` (`self.TowerHead`) 0 (`local.Material `)))

(fn `UserConstructionScript`)