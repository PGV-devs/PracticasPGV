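; Parent Blueprint for tower projectiles that deal damage to spline-following enemies.
; It records its spawn location and destroys itself once it travels beyond its range.
; Its sphere overlap casts to the parent enemy class, so any enemy type counts, then applies damage once and destroys the projectile.
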(event `self.ReceiveBeginPlay`
  (set `self.StartLocation` (`self.K2_GetActorLocation`)))

(event `self.ReceiveTick`
  (params (DeltaSeconds :type "Float (single-precision)"))
  (if (> (`KismetMathLibrary.VSize` (- (`self.StartLocation`) (`self.K2_GetActorLocation`))) (`self.ProjectileRange`))
    (`/Engine/EditorBlueprintResources/StandardMacros.DoOnce` false
      (:`Completed`
        (`self.K2_DestroyActor`)))))

(event `self.Sphere.OnComponentBeginOverlap`
  (params (OverlappedComponent :type "PrimitiveComponent Object Reference") (OtherActor :type "Actor Object Reference") (OtherComp :type "PrimitiveComponent Object Reference") (OtherBodyIndex :type Integer) (bFromSweep :type Boolean) (SweepResult :type "HitResult Structure (by ref)"))
  (bind _ascharacter_spline_parent (cast `/Game/Blueprints/Enemies/EnemySPLine_Parent` OtherActor)) ; Elige como objetivo cualquier tipo de bicho\nya que castea al blueprint padre de los bichos
  (`/Engine/EditorBlueprintResources/StandardMacros.DoOnce` false
    (:`Completed`
      (`GameplayStatics.ApplyDamage` _ascharacter_spline_parent (`self.Damage`) null self)
      (`self.K2_DestroyActor`))))

(fn `UserConstructionScript`)