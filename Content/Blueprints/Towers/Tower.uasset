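; Defense tower actor that targets the nearest EnemySPLine_Child in its shoot area, with HP, a health widget and destruction at zero.
; Tick reselects the target, a gated delay loop rotates body yaw and head pitch toward it, and a refire timeline paces shots.
; Projectile type sets the spawned class and pitch offset for parabolic or straight shots.
; Holding right mouse traces the predicted arc as a debug drawing.
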(event `ContinueFiring`
  ;[1 1 1] Firing at target time events
  (if (`self.CanShoot`)
    (`/Engine/EditorBlueprintResources/StandardMacros.IsValid` (`self.SelectedTarget`)
      (:`Is Valid`
        (if (== (`TimelineComponent.GetPlaybackPosition` (`self.TurrentRefire`)) 0.0) :!label _label
          (`self.shootProjectile`)
          (`Timeline|TurrentRefire` :!label _label_2
            (:`Finished`
              (`self.ResetFireTimeline`)
              (`self.ContinueFiring`))))))))

(event `StartFiring`
  ;[1 1 1] Firing at target time events
  (set `self.CanShoot` true)
  (`TimelineComponent.SetTimelineLength` (`self.TurrentRefire`) (`self.RefireDelay`))
  (goto _label))

(event `ResetFireTimeline`
  ;[1 1 1] Firing at target time events
  (`|ExecutionSequence`
    (:`then_0`
      (goto _label_2 :!via `Stop`))
    (:`then_1`
      (goto _label_2 :!via `SetNewTime`))))

(event `StopFiring`
  ;[1 1 1] Firing at target time events
  (`self.ResetFireTimeline`)
  (set `self.CanShoot` false))

(event `self.ReceiveBeginPlay`
  (set `self.CurrentHP` (`self.HP_MAX`))
  (`self.EnableInput` (`GameplayStatics.GetPlayerController` 0))
  (bind _aswb_hpenemy (cast `/Game/HUD/WB_HPEnemy` (`WidgetComponent.GetUserWidgetObject` (`self.WidgetHPEnemy`))))
  (set `/Game/HUD/WB_HPEnemy.Parent Object` self _aswb_hpenemy))

(event `SelectTarget`
  ;[1 1 1] Select random target in shoot area
  (if (!= (`KismetArrayLibrary.Array_Length` (`self.TargetsInRange`)) 0)
    (bind _asenemy_spline_child (cast `/Game/Blueprints/Enemies/EnemySPLine_Child` (`.ReturnValue` (`GameplayStatics.FindNearestActor` (`self.K2_GetActorLocation`) (`self.TargetsInRange`)))))
    (set `self.SelectedTarget` _asenemy_spline_child)
    (`self.BeginAim`)
    (if (not (`self.is Firing`))
      (`self.StartFiring`)
      (set `self.is Firing` true))))

(event `ContinueAim`
  ;[1 1 1] Rotate Turret to Aim Target
  (`/Engine/EditorBlueprintResources/StandardMacros.IsValid` (`self.SelectedTarget`)
    (:`Is Valid`
      (`/Engine/EditorBlueprintResources/StandardMacros.Gate` true :!label _label_3
        (:`Exit`
          (`/Engine/EditorBlueprintResources/StandardMacros.IsValid` (`self.SelectedTarget`)
            (:`Is Valid`
              (bind _orientation (`self.updateOrientationToTarget` (`self.SelectedTarget`)))
              (`self.rotateTowardsTarget` _orientation)
              (`KismetSystemLibrary.Delay` (`GameplayStatics.GetWorldDeltaSeconds`))
              (`self.ContinueAim`))
            (:`Is Not Valid`
              (`self.CancelAim` :!label _label_4)
              (`self.BeginResetAim`))))))
    (:`Is Not Valid`
      (goto _label_4))))

(event `BeginAim`
  ;[1 1 1] Rotate Turret to Aim Target
  (`|ExecutionSequence`
    (:`then_0`
      (goto _label_3 :!via `Open`))
    (:`then_1`
      (goto _label_3))))

(event `self.ReceiveTick`
  (params (DeltaSeconds :type "Float (single-precision)"))
  ;[1 1 1] (DEBUG)
  ;;[1 1 1] Show trayectory
  (`self.SelectTarget`)
  (`/Engine/EditorBlueprintResources/StandardMacros.Gate` true :!label _label_5
    (:`Exit`
      (`self.DrawProjectileTrayectory`))))

(event `CancelAim`
  ;[1 1 1] Rotate Turret to Aim Target
  (goto _label_3 :!via `Close`))

(event `self.ShootArea.OnComponentBeginOverlap`
  (params (OverlappedComponent :type "PrimitiveComponent Object Reference") (OtherActor :type "Actor Object Reference") (OtherComp :type "PrimitiveComponent Object Reference") (OtherBodyIndex :type Integer) (bFromSweep :type Boolean) (SweepResult :type "HitResult Structure (by ref)"))
  ;[1 1 1] Adds target to target list if not already
  (bind _asenemy_spline_child (cast `/Game/Blueprints/Enemies/EnemySPLine_Child` OtherActor))
  (`KismetArrayLibrary.Array_Add` (`self.TargetsInRange`) _asenemy_spline_child))

(event `BeginResetAim`
  ;[1 1 1] Rotate Turret to Aim Target
  (`self.resetAim`))

(event `Key|RightMouseButton`
  (params (Key :type "Key Structure"))
  ;[1 1 1] (DEBUG)
  (:`Pressed`
    (goto _label_5 :!via `Open`))
  (:`Released`
    (goto _label_5 :!via `Close`)))

(event `self.ShootArea.OnComponentEndOverlap`
  (params (OverlappedComponent :type "PrimitiveComponent Object Reference") (OtherActor :type "Actor Object Reference") (OtherComp :type "PrimitiveComponent Object Reference") (OtherBodyIndex :type Integer))
  ;[1 1 1] Remove a target if it exists the shooting area
  (bind _asenemy_spline_child (cast `/Game/Blueprints/Enemies/EnemySPLine_Child` OtherActor))
  (if (`KismetArrayLibrary.Array_Contains` (`self.TargetsInRange`) _asenemy_spline_child)
    (`KismetArrayLibrary.Array_RemoveItem` (`self.TargetsInRange`) _asenemy_spline_child)
    (if (== _asenemy_spline_child (`self.SelectedTarget`))
      (set `self.SelectedTarget` null)
      (if (== (`KismetArrayLibrary.Array_Length` (`self.TargetsInRange`)) 0)
        (set `self.is Firing` false)
        (`self.StopFiring`)))))

(event `DrawProjectileTrayectory`
  (bind _returnvalue (`SceneComponent.K2_GetComponentRotation` (`self.TowerHead`)))
  (bind _returnvalue_2 (+ (`SceneComponent.K2_GetComponentLocation` (`self.TowerHead`)) (`KismetMathLibrary.GreaterGreater_VectorRotator` (80.0 0.0 0.0) _returnvalue)))
  ;[1 1 1] Make Projectile trayectory
  (set `self.StartLocation` _returnvalue_2)
  (set `self.InitialVelocity` (`KismetMathLibrary.TransformDirection` (`KismetMathLibrary.MakeTransform` _returnvalue_2 _returnvalue (0.5 0.5 0.5)) (`self.InitialLocalVelocity`)))
  (for _index (range (+ (`KismetMathLibrary.FFloor` (/ (`self.PathLifeTime`) (`self.TimeInterval`))) 1)) :!label _label_6
    (bind (_point1 _point2) (`self.getSegmentAtTime` (`self.StartLocation`) (`self.InitialVelocity`) (0.0 0.0 -980.0) (* _index (`self.TimeInterval`)) (* (+ _index 1) (`self.TimeInterval`))))
    (bind (_outhit _returnvalue_3) (`KismetSystemLibrary.LineTraceSingle` :`Start` _point1 :`End` _point2 :`TraceChannel` "TraceTypeQuery1" :`bTraceComplex` true :`DrawDebugType` "ForOneFrame"))
    (if _returnvalue_3
      (`self.BreakDrawingLoop`))))

(event `BreakDrawingLoop`
  ;[1 1 1] Make Projectile trayectory
  (goto _label_6 :!via `Break`))

(fn `die`
  (`self.K2_DestroyActor`))

(fn `getProyectileClass`
  (returns (NewParam :type "Actor Class Reference"))
  (switch `/Game/Blueprints/Towers/Projectiles/ProjectileType` (`self.ProjectileType`)
    (:`NewEnumerator0`
      (return "/Game/Blueprints/Towers/Projectiles/ParabolicBullet.ParabolicBullet_C"))
    (:`NewEnumerator1`
      (return "/Game/Blueprints/Towers/Projectiles/StraightLineBullet.StraightLineBullet_C"))))

(fn `getSegmentAtTime`
  (params (StartLocation :type "Vector Structure") (InitialVelocity :type "Vector Structure") (Gravity :type "Vector Structure") (Time1 :type "Float (double-precision)") (Time2 :type "Float (double-precision)"))
  (returns (Point1 :type "Vector Structure") (Point2 :type "Vector Structure"))
  (return (+ StartLocation (* InitialVelocity Time1) (* Gravity (* Time1 Time1 0.5))) (+ StartLocation (* InitialVelocity Time2) (* Gravity (* Time2 Time2 0.5)))))

(fn `receiveDamage`
  (params (damage :type "Float (double-precision)"))
  (locals (NewHP :type "Float (double-precision)" :default 0.0))
  (bind _output_get (set `local.NewHP` (- (`self.CurrentHP`) damage)))
  (if (<= _output_get 0.0)
    (set `self.CurrentHP` 0.0)
    (`self.die`)
    (else
      (set `self.CurrentHP` (`local.NewHP`)))))

(fn `resetAim`
  (`SceneComponent.K2_SetRelativeRotation` (`self.TowerBody`) (`KismetMathLibrary.RInterpTo_Constant` (`SceneComponent.RelativeRotation` (`self.TowerBody`)) (struct) (`GameplayStatics.GetWorldDeltaSeconds`) 100.0) false false)
  (`SceneComponent.K2_SetRelativeRotation` (`self.TowerHead`) (`KismetMathLibrary.RInterpTo_Constant` (`SceneComponent.RelativeRotation` (`self.TowerHead`)) (struct) (`GameplayStatics.GetWorldDeltaSeconds`) 100.0) false false))

(fn `rotateTowardsTarget`
  (params (Orientation :type "Rotator Structure"))
  (locals (orientationToTarget :type "Rotator Structure") (lookUpOffset :type "Float (double-precision)") (rotateSpeed :type "Float (double-precision)" :default 150.0))
  (bind (_orientationtotarget_roll _orientationtotarget_pitch _orientationtotarget_yaw) (`KismetMathLibrary.BreakRotator` (`local.orientationToTarget`)))
  (bind (_orientationtotarget_roll_2 _orientationtotarget_pitch_2) (`KismetMathLibrary.BreakRotator` (`local.orientationToTarget`)))
  (set `local.orientationToTarget` Orientation)
  (switch `/Game/Blueprints/Towers/Projectiles/ProjectileType` (`self.ProjectileType`)
    (:`NewEnumerator0`
      (set `local.lookUpOffset` 20.0))
    (:`NewEnumerator1`
      (set `local.lookUpOffset` 2.0)))
  (`SceneComponent.K2_SetRelativeRotation` (`self.TowerBody`) (`KismetMathLibrary.RInterpTo_Constant` (`SceneComponent.RelativeRotation` (`self.TowerBody`)) (`KismetMathLibrary.MakeRotator` 0.0 0.0 _orientationtotarget_yaw) (`GameplayStatics.GetWorldDeltaSeconds`) (`local.rotateSpeed`)) false false)
  (`SceneComponent.K2_SetRelativeRotation` (`self.TowerHead`) (`KismetMathLibrary.RInterpTo_Constant` (`SceneComponent.RelativeRotation` (`self.TowerHead`)) (`KismetMathLibrary.MakeRotator` 0.0 (`KismetMathLibrary.ClampAngle` (+ _orientationtotarget_pitch_2 (`local.lookUpOffset`)) -20.0 200.0)) (`GameplayStatics.GetWorldDeltaSeconds`) (`local.rotateSpeed`)) false false))

(fn `shootProjectile`
  (locals (Proyectile :type "/Game/Blueprints/Towers/Projectiles/Projectile_Parent Object Reference"))
  (bind _returnvalue (`SceneComponent.K2_GetComponentRotation` (`self.TowerHead`)))
  (bind _projectilemovement (`/Game/Blueprints/Towers/Projectiles/Projectile_Parent.ProjectileMovement` (`local.Proyectile`)))
  (bind _newparam (`self.getProyectileClass`))
  (bind _returnvalue_2 (`|SpawnActorFromClass` _newparam (`KismetMathLibrary.MakeTransform` (+ (`SceneComponent.K2_GetComponentLocation` (`self.TowerHead`)) (`KismetMathLibrary.GreaterGreater_VectorRotator` (`self.TowerHeadOffset`) _returnvalue)) _returnvalue (1.5 1.5 1.5)) "Undefined" "OverrideRootScale" null null))
  (bind _asprojectile_parent (cast `/Game/Blueprints/Towers/Projectiles/Projectile_Parent` _returnvalue_2))
  (bind _output_get (set `local.Proyectile` _asprojectile_parent))
  (set `/Game/Blueprints/Towers/Projectiles/Projectile_Parent.Damage` (`self.Damage`) _output_get)
  (`/Engine/EditorBlueprintResources/StandardMacros.IsValid` _projectilemovement
    (:`Is Valid`
      (`ProjectileMovementComponent.SetVelocityInLocalSpace` _projectilemovement (`self.InitialLocalVelocity`)))))

(fn `updateLerpAlphaValue`)

(fn `updateOrientationToTarget`
  (params (Objetive :type "Actor Object Reference"))
  (returns (Orientation :type "Rotator Structure"))
  ;[1 1 1] Returns where the turret has to look at
  (return (`KismetMathLibrary.MakeRotFromX` (`KismetMathLibrary.InverseTransformDirection` (`self.GetTransform`) (- (`self.K2_GetActorLocation` Objetive) (`SceneComponent.K2_GetComponentLocation` (`self.TowerHead`)))))))

(fn `UserConstructionScript`)