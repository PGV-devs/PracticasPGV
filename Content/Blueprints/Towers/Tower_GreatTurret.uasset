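; Great turret tower, a Blueprint variant that tunes an inherited tower through stat overrides alone.
; Its construction script runs the parent's, then selects a projectile type, boosts bullet speed and sets refire delay, muzzle offset and hit points.
; The event graph adds no behavior of its own, only calling the parent on BeginPlay and leaving Tick and overlap events disabled.
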(event `self.ReceiveBeginPlay`
  (`parent.ReceiveBeginPlay`))

(fn `UserConstructionScript`
  (`parent.UserConstructionScript`)
  (set `self.ProjectileType` "NewEnumerator1")
  ;[1 1 1] Increase Bullet speed
  (set `self.InitialLocalVelocity` (+ (`self.InitialLocalVelocity`) (5000.0 0.0 0.0)))
  ;[1 1 1] Increase cadency
  (set `self.RefireDelay` 0.5)
  ;[1 1 1] Adjust projectile spawn location
  (set `self.TowerHeadOffset` (900.0 0.0 0.0))
  ;[1 1 1] Number of hits it can take
  (set `self.HealthPoints` 15))