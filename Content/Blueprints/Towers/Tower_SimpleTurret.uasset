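; Simple turret tower Blueprint, a child of a parent tower class that supplies the actual turret behavior.
; Its Construction Script overrides inherited settings for projectile type, muzzle velocity, fire rate, spawn offset, health and damage, then calls the parent construction script.
; The event graph only forwards BeginPlay to the parent; Tick and overlap events are disabled.
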(event `self.ReceiveBeginPlay`
  (`parent.ReceiveBeginPlay`))

(fn `UserConstructionScript`
  (set `self.ProjectileType` "NewEnumerator1")
  ;[1 1 1] Set Bullet speed
  (set `self.InitialLocalVelocity` (4500.0 0.0 0.0))
  ;[1 1 1] Increase cadency
  (set `self.RefireDelay` 0.5)
  ;[1 1 1] Adjust projectile spawn location
  (set `self.TowerHeadOffset` (600.0 0.0 0.0))
  ;[1 1 1] Number of hits it can take
  (set `self.HealthPoints` 100)
  (set `self.Damage` 25.0)
  (`parent.UserConstructionScript`))